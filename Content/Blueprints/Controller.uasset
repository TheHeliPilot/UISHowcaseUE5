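; Controller Blueprint that opens the main menu and manages the player inventory screen.
; BeginPlay shows the main menu with UI-only input and a visible cursor, then creates the inventory widget once and stores it off-screen.
; ToggleInventory, gated by IsInGame, uses a FlipFlop to add or remove that widget without changing input mode.
; Unconnected leftover nodes for a player UI and alternative inventory setup never run.
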(event `self.ReceiveBeginPlay`
  (bind _returnvalue (`GameplayStatics.GetPlayerController` 0))
  (`|ExecutionSequence`
    (:`then_0`
      (bind _returnvalue_2 (`|CreateWidget` "/Game/Blueprints/WB_MainMenu.WB_MainMenu_C" _returnvalue))
      (`UserWidget.AddToViewport` _returnvalue_2 0)
      (`WidgetBlueprintLibrary.SetInputMode_UIOnlyEx` _returnvalue _returnvalue_2)
      (set `PlayerController.bShowMouseCursor` true _returnvalue))
    (:`then_1`
      (bind _returnvalue_3 (`|CreateWidget` "/Game/Blueprints/WB_PlayerInventory.WB_PlayerInventory_C" _returnvalue))
      (bind _output_get (set `self.Inventory` _returnvalue_3)))))

(event `ToggleInventory`
  (if (`self.IsInGame`)
    (`/Engine/EditorBlueprintResources/StandardMacros.FlipFlop`
      (:`A`
        (`UserWidget.AddToViewport` (stale `self.ReceiveBeginPlay` _output_get) 10))
      (:`B`
        (`Widget.RemoveFromParent` (stale `self.ReceiveBeginPlay` _output_get))))))

(fn `UserConstructionScript`)